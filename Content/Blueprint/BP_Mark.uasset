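; BP_Mark is an input-driven actor that turns, flags movement, and puts the Net_HUD widget on screen at begin play.
; Q and E call Turn with different direction flags, F sets NeedMove, and Escape quits the game.
; The graph only issues these requests; the turn and movement logic is not in it.
; A debug loop printing TriggerStats is left unconnected, and Tick is empty.
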(event `Key|Q`
  (params (Key :type "Key Structure"))
  (:`Pressed`
    (`self.Turn` true true)))

(event `Key|E`
  (params (Key :type "Key Structure"))
  (:`Pressed`
    (`self.Turn` false true)))

(event `Key|Escape`
  (params (Key :type "Key Structure"))
  (:`Pressed`
    (`KismetSystemLibrary.QuitGame` null "Quit")))

(event `Key|F`
  (params (Key :type "Key Structure"))
  (:`Pressed`
    (set `self.NeedMove` true)))

(event `self.ReceiveBeginPlay`
  (bind _returnvalue (`|CreateWidget` "/Game/Blueprint/Net_HUD.Net_HUD_C"))
  (`UserWidget.AddToViewport` _returnvalue 0))

(event `self.ReceiveTick`
  (params (DeltaSeconds :type "Float (single-precision)")))

(fn `UserConstructionScript`)